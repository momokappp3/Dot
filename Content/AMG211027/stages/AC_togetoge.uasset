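; AC_togetoge is a spike trap actor that moves a cone when the main character comes near and shows game over on contact.
; Entering the Sphere trigger plays a timeline that drives the Cone's relative Z location, and leaving reverses it.
; Overlapping the Cone creates the WI_gameover widget and adds it to the viewport.
; Both triggers respond only to an exact CH_mainchar class match.
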(event OnComponentBeginOverlap(Cone)
  (params (OverlappedComponent :type Primitive%20Component%20Object%20Reference) (OtherActor :type Actor%20Object%20Reference) (OtherComp :type Primitive%20Component%20Object%20Reference) (OtherBodyIndex :type Integer) (bFromSweep :type Boolean) (SweepResult :type Hit%20Result%20Structure%20%28by%20ref%29))
  (if (== (Utilities|GetClass OtherActor) "/Game/AMG211027/stages/CH_mainchar.CH_mainchar_C")
    (bind _returnvalue (UserInterface|CreateWidget "/Game/AMG211027/gameover/WI_gameover.WI_gameover_C"))
    (UserInterface|Viewport|AddtoViewport _returnvalue 0)))

(event OnComponentBeginOverlap(Sphere)
  (params (OverlappedComponent :type Primitive%20Component%20Object%20Reference) (OtherActor :type Actor%20Object%20Reference) (OtherComp :type Primitive%20Component%20Object%20Reference) (OtherBodyIndex :type Integer) (bFromSweep :type Boolean) (SweepResult :type Hit%20Result%20Structure%20%28by%20ref%29))
  (if (== (Utilities|GetClass OtherActor) "/Game/AMG211027/stages/CH_mainchar.CH_mainchar_C")
    (bind _新規track_1 (Timeline|togetogeTimeline Play)
      (:Update
        (Transformation|SetRelativeLocation (Variables|Default|GetCone) (Math|Vector|MakeVector 0.0 0.0 _新規track_1) false false)))))

(event OnComponentEndOverlap(Sphere)
  (params (OverlappedComponent :type Primitive%20Component%20Object%20Reference) (OtherActor :type Actor%20Object%20Reference) (OtherComp :type Primitive%20Component%20Object%20Reference) (OtherBodyIndex :type Integer))
  (if (== (Utilities|GetClass OtherActor) "/Game/AMG211027/stages/CH_mainchar.CH_mainchar_C")
    (bind _新規track_1 (Timeline|togetogeTimeline Reverse)
      (:Update
        (Transformation|SetRelativeLocation (Variables|Default|GetCone) (Math|Vector|MakeVector 0.0 0.0 _新規track_1) false false)))))

(event EventBeginPlay)

(event Collision|EventActorBeginOverlap
  (params (OtherActor :type Actor%20Object%20Reference)))

(event EventTick
  (params (DeltaSeconds :type Float%20%28single-precision%29)))

(fn ConstructionScript)