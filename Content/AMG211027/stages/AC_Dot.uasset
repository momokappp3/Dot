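; Collectible dot placed in stages that bobs or moves vertically and reports to the game mode when picked up.
; On BeginPlay, a timeline drives the sphere's relative Z, and the dot calls IncrementDot on GM_Common.
; Any actor overlap while the sphere is visible hides it and calls IncrementDot again.
; The visibility flag doubles as the collected state, since the actor is never destroyed.
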(event EventBeginPlay
  (Utilities|FlowControl|Sequence
    (:then_0
      (bind _新規track_0 (Timeline|dotTimeline Play)
        (:Update
          (Transformation|SetRelativeLocation (Variables|Default|GetSphere) (Math|Vector|MakeVector 0.0 0.0 _新規track_0) false false))))
    (:then_1
      (bind _asgm_common (Utilities|Casting|CastToGM_Common (Game|GetGameMode)))
      (Default|IncrementDot _asgm_common))))

(event Collision|EventActorBeginOverlap
  (params (OtherActor :type Actor%20Object%20Reference))
  (bind _sphere (Variables|Default|GetSphere))
  (if (Variables|/Script/Engine.SceneComponent|GetbVisible _sphere)
    (Rendering|SetVisibility _sphere false false)
    (bind _asgm_common (Utilities|Casting|CastToGM_Common (Game|GetGameMode)))
    (Default|IncrementDot _asgm_common)))

(event EventTick
  (params (DeltaSeconds :type Float%20%28single-precision%29)))

(fn ConstructionScript)